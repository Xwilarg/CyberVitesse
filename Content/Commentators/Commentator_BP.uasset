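; Commentator Blueprint that gives a commentator camera views of the game.
; BeginPlay sets player 0's view target to the first camera in the CameraManager's list, while the Cam1 input passes the first CameraActor found to CallApplyCameraChange.
; The DisplayName input prints debug text identifying the commentator and the number of commentators.
; FillActorsPawnArray gathers Player_BP actors into PlayerPawns but is not called within this Blueprint.
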(event EventBeginPlay
  (bind _outactors (Actor|GetAllActorsOfClass "/Game/CameraManager.CameraManager_C"))
  (Game|Player|SetViewTargetwithBlend (Game|GetPlayerController 0) (Utilities|ResolveSoftReference (Utilities|Array|Get(acopy) (Variables|/Game/CameraManager.CameraManager_C|GetCameraLists (Utilities|Array|Get(acopy) _outactors)))) 0.0 "VTBlend_Linear" 0.0 false))

(event Collision|EventActorBeginOverlap
  (params (OtherActor :type Actor%20Object%20Reference)))

(event EventTick
  (params (DeltaSeconds :type Float%20%28single-precision%29)))

(event Input|ActionEvents|InputActionCam1
  (params (Key :type Key%20Structure))
  (:Pressed
    (bind _outactors (Actor|GetAllActorsOfClass "/Script/Engine.CameraActor"))
    (Default|CallApplyCameraChange (Utilities|Array|Get(acopy) _outactors))))

(event Input|ActionEvents|InputActionDisplayName
  (params (Key :type Key%20Structure))
  (:Pressed
    (Development|PrintString "Je suis le commentateur" true true "(R=0.000000,G=0.660000,B=1.000000,A=1.000000)" 15.0)
    (bind _outactors (Actor|GetAllActorsOfClass "Commentator_BP_C"))
    (Development|PrintString (Utilities|String|ToString(Integer) (Utilities|Array|Length _outactors)) true true "(R=0.000000,G=0.660000,B=1.000000,A=1.000000)" 1e+01)))

(fn ConstructionScript)

(fn FillActorsPawnArray
  (bind _outactors (Actor|GetAllActorsOfClass "/Game/Player/Player_BP.Player_BP_C"))
  (for _array_element _outactors
    (Utilities|Array|Add (Variables|Default|GetPlayerPawns) _array_element)))