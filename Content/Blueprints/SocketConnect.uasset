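; SocketConnect is an actor that opens a WebSocket to a hardcoded LAN server on BeginPlay and recolors its Cube from received messages.
; The socket is stored on NetworkGameInstance so it survives level loading.
; On connect it sends an identifying text, then prints incoming data and swaps the Cube material for Red or Green.
; Close and error handlers exist, but their bindings never run.
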(event Custom|OnConnectComplete_Event_0
  (Development|PrintString "WebSocket Connect Success")
  (Class|WebSocketBase|SendText (stale EventBeginPlay _output_get) "UnrealSocket")
  (EventDispatchers|AssignOnReceiveData (stale EventBeginPlay _output_get) (delegate Custom|OnReceiveData_Event_0)))

(event Custom|CustomEvent_1
  (Development|PrintString "Closed!!!!" true true "(R=0.000000,G=0.660000,B=1.000000,A=1.000000)" 1e+03))

(event Custom|CustomEvent_0
  (params (error :type String))
  (Development|PrintString error))

(event Custom|OnReceiveData_Event_0
  (params (data :type String))
  (bind _cube (Variables|Default|GetCube))
  (Development|PrintString data true true "(R=1.000000,G=0.330410,B=0.390180,A=1.000000)")
  (switch string data
    (:Red
      (Rendering|Material|SetMaterial _cube 0 "/Game/StarterContent/Materials/M_Wood_Floor_Walnut_Polished.M_Wood_Floor_Walnut_Polished"))
    (:Green
      (Rendering|Material|SetMaterial _cube 0 "/Game/StarterContent/Materials/M_Ground_Moss.M_Ground_Moss"))))

(event EventBeginPlay
  ;[1 1 1] Save WebSocket to GameInstance, so the socket will not destroy after level loading
  (bind _returnvalue (Class|WebSocketBlueprintLibrary|Connect "ws://192.168.1.20:1234"))
  (bind _asnetwork_game_instance (Utilities|Casting|CastToNetworkGameInstance (Game|GetGameInstance)))
  (bind _output_get (Variables|/Game/Blueprints/NetworkGameInstance.NetworkGameInstance_C|SetSocket _asnetwork_game_instance _returnvalue))
  (Rendering|Material|SetMaterial (Variables|Default|GetCube) 0 "/Game/StarterContent/Props/Materials/M_TableRound.M_TableRound")
  (EventDispatchers|AssignOnConnectComplete _output_get (delegate Custom|OnConnectComplete_Event_0)))

(event Collision|EventActorBeginOverlap
  (params (OtherActor :type Actor%20Object%20Reference)))

(event EventTick
  (params (DeltaSeconds :type Float%20%28single-precision%29)))

(fn ConstructionScript)