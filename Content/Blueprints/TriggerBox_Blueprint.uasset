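; Trigger volume with a torus ring that reacts to a Drone overlapping it.
; Entering the collision component finds the first SocketConnect actor in the level and calls RequestShaking on it with the trigger's first actor tag as a string.
; Overlapping the torus prints a debug message and sets a Passed flag, so that response fires only once.
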(event OnComponentBeginOverlap(CollisionComponent)
  (params (OverlappedComponent :type Primitive%20Component%20Object%20Reference) (OtherActor :type Actor%20Object%20Reference) (OtherComp :type Primitive%20Component%20Object%20Reference) (OtherBodyIndex :type Integer) (bFromSweep :type Boolean) (SweepResult :type Hit%20Result%20Structure%20%28by%20ref%29))
  (Utilities|Casting|CastToDrone OtherActor)
  (bind _outactors (Actor|GetAllActorsOfClass "/Game/Blueprints/SocketConnect.SocketConnect_C"))
  (Default|RequestShaking (Utilities|Array|Get(acopy) _outactors) (Utilities|String|ToString(Name) (Utilities|Array|Get(acopy) (Variables|Actor|GetTags self)))))

(event OnComponentBeginOverlap(Torus)
  (params (OverlappedComponent :type Primitive%20Component%20Object%20Reference) (OtherActor :type Actor%20Object%20Reference) (OtherComp :type Primitive%20Component%20Object%20Reference) (OtherBodyIndex :type Integer) (bFromSweep :type Boolean) (SweepResult :type Hit%20Result%20Structure%20%28by%20ref%29))
  (if (not (Variables|Default|GetPassed))
    (Utilities|Casting|CastToDrone OtherActor)
    (Development|PrintString "Going through")
    (Variables|Default|SetPassed true)))

(event EventBeginPlay)

(event Collision|EventActorBeginOverlap
  (params (OtherActor :type Actor%20Object%20Reference)))

(event EventTick
  (params (DeltaSeconds :type Float%20%28single-precision%29)))

(fn ConstructionScript)