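; Score actor that tallies Red and Blue votes received over a WebSocket and flags a winner.
; While active, Tick clears the tallies if Reset is set and opens a new socket connection every frame, storing it on NetworkGameInstance.
; On connect it sends text and binds receipt, where Red or Blue messages increment votes.
; When inactive, Tick sets RedWinner if Red has fewer votes, otherwise BlueWinner.
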(event Custom|OnCommandComplete
  (Class|WebSocketBase|SendText (stale EventTick _output_get) "UnrealSocket")
  (EventDispatchers|BindEventtoOnReceiveData (stale EventTick _output_get) (delegate Custom|OnRecienveData%20EnventOne))
  (Class|WebSocketBase|SendText (stale EventTick _output_get) (stale Custom|OnRecienveData%20EnventOne data)))

(event Custom|OnRecienveData%20EnventOne
  (params (data :type String))
  (switch string data
    (:Red
      (bind _result (Math|Integer|IncrementInt (Variables|Default|GetRedVote))
        (:%20%20
          (Variables|Default|SetRedVote _result)
          (Variables|Default|SetReset false))))
    (:Blue
      (bind _result_2 (Math|Integer|IncrementInt (Variables|Default|GetBlueVote))
        (:%20%20
          (Variables|Default|SetBlueVote _result_2)
          (Variables|Default|SetReset false))))))

(event EventTick
  (params (DeltaSeconds :type Float%20%28single-precision%29))
  (if (Variables|Default|GetIsActive)
    (if (Variables|Default|GetReset)
      (Variables|Default|SetRedWinner false)
      (Variables|Default|SetBlueWinner false)
      (Variables|Default|SetBlueVote 0)
      (Variables|Default|SetRedVote 0))
    (bind _returnvalue (Class|WebSocketBlueprintLibrary|Connect "ws://192.168.1.20:1234"))
    (bind _asnetwork_game_instance (Utilities|Casting|CastToNetworkGameInstance (Game|GetGameInstance)))
    (bind _output_get (Variables|/Game/Blueprints/NetworkGameInstance.NetworkGameInstance_C|SetSocket _asnetwork_game_instance _returnvalue))
    (EventDispatchers|BindEventtoOnConnectComplete _output_get (delegate Custom|OnCommandComplete))
    (elif (< (Variables|Default|GetRedVote) (Variables|Default|GetBlueVote))
      (Variables|Default|SetRedWinner true)
      (else
        (Variables|Default|SetBlueWinner true)))))

(fn ConstructionScript)