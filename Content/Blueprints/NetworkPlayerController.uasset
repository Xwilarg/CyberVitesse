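; Player controller for networked play that sets up the in-game HUD and requests its player's actor from the game mode.
; ClientPostLogin runs the UI setup, then calls SpawnActor on NetworkGameMode with itself, if that cast succeeds.
; For local controllers only, SetupIngameUI adds VRUi to the viewport when player pawn 0 is a Player_BP, otherwise BasicUI for commentators.
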(event Custom|ClientPostLogin
  (CallFunction|SetupIngameUI)
  (bind _asnetwork_game_mode (Utilities|Casting|CastToNetworkGameMode (Game|GetGameMode)))
  (Default|SpawnActor _asnetwork_game_mode self))

(event EventBeginPlay)

(event EventTick
  (params (DeltaSeconds :type Float%20%28single-precision%29)))

(fn ConstructionScript)

(fn SetupIngameUI
  (bind _self self)
  (if (Pawn|IsLocalPlayerController)
    (Utilities|Casting|CastToPlayer_BP (Game|Player|GetPlayerPawn 0)
      (:then
        (bind _returnvalue (UserInterface|CreateWidget "/Game/Blueprints/Widgets/VRUi.VRUi_C" _self))
        (bind _output_get (Variables|Default|SetHUDWidget _returnvalue))
        (UserInterface|Viewport|AddtoViewport _output_get 0))
      (:CastFailed
        ;[1 1 1] Create commentator UI
        (bind _returnvalue_2 (UserInterface|CreateWidget "/Game/BasicUI.BasicUI_C" _self))
        (bind _output_get_2 (Variables|Default|SetHUDWidget _returnvalue_2))
        (UserInterface|Viewport|AddtoViewport _output_get_2 0)))))