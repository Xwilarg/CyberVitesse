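; Game instance that hosts and joins LAN multiplayer sessions and shows the main menu.
; StartNewGame swaps the calling widget for a loading screen, creates a session and opens TrackLevel as a listen server.
; StartLooking repeats searches until results appear, stores the first and calls an empty EnableJoinSession event, but its call in StartGame is disconnected.
; FindSession runs its own search and joins the first result.
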(event Custom|StartLooking
  ;[1 1 1] Look For Session
  (bind _results (|FindSessions (Game|GetPlayerController 0) 20 true)
    (:OnSuccess
      (if (>= (Utilities|Array|Length _results) 1)
        (CallFunction|EnableJoinSession)
        (Variables|Default|SetAvailableGameSession (Utilities|Array|Get(acopy) _results))
        (Development|PrintString (Utilities|String|ToString(Integer) (Utilities|Array|Length _results)))
        (else
          (CallFunction|StartLooking))))
    (:OnFailure
      (Development|PrintString "failed to find session"))))

(event Custom|EnableJoinSession)

(event Custom|StartNewGame
  (params (CallingWidget :type Widget%20Object%20Reference))
  ;[1 1 1] Create a new session
  (Variables|Default|SetCurrentWidget CallingWidget)
  (Widget|RemovefromParent CallingWidget)
  (bind _returnvalue (UserInterface|CreateWidget "/Game/Blueprints/Widgets/LoadingScreen.LoadingScreen_C"))
  (UserInterface|Viewport|AddtoViewport _returnvalue 0)
  (|Session (Game|GetPlayerController 0) 3 true
    (:OnSuccess
      (Utilities|FlowControl|Delay 0.5)
      (Game|OpenLevel(byName) "TrackLevel" true "listen"))))

(event Custom|FindSession
  (bind _results (|FindSessions (Game|GetPlayerController 0) 20 true)
    (:OnSuccess
      (if (>= (Utilities|Array|Length _results) 1)
        (|JoinSession (Game|GetPlayerController 0) (Utilities|Array|Get(acopy) _results))))))

(event Custom|ShowMainMenu
  (bind _returnvalue (Game|GetPlayerController 0))
  (bind _returnvalue_2 (UserInterface|CreateWidget "/Game/Blueprints/Widgets/WidgetMenu.WidgetMenu_C" _returnvalue))
  (Input|SetInputModeGameandUI _returnvalue _returnvalue_2 "DoNotLock" true)
  (UserInterface|Viewport|AddtoViewport _returnvalue_2 0))